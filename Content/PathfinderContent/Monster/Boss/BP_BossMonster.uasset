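; Stationary boss monster, driven by an AI controller and blackboard, that launches projectiles and minions at the player.
; BeginPlay initializes its stat component, disables movement and caches the player.
; Damage updates the blackboard hit flag, spawns impact effects and reduces health, destroying the boss with sound and effects on death.
; Attack functions lob boilers and mini bosses using ballistic velocity solved from a launch angle, or fire boxes straight toward the player.
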(event `self.ReceiveBeginPlay`
  (`parent.ReceiveBeginPlay`)
  (`/Game/PathfinderContent/Component/BPC_StatSystem.InitializeEnemyState` (`self.BPC_StatSystem`) 1000.0)
  (`CharacterMovementComponent.DisableMovement` (`self.CharacterMovement`))
  (bind _asbp_player (cast `/Game/PathfinderContent/Player/BP_Player` (`GameplayStatics.GetPlayerCharacter` 0)))
  (set `self.PlayerCharacter` _asbp_player))

(event `self.AICollision.OnComponentBeginOverlap`
  (params (OverlappedComponent :type "PrimitiveComponent Object Reference") (OtherActor :type "Actor Object Reference") (OtherComp :type "PrimitiveComponent Object Reference") (OtherBodyIndex :type Integer) (bFromSweep :type Boolean) (SweepResult :type "HitResult Structure (by ref)"))
  ;[1 1 1] AI의 플레이어 감지(플레이어와 AIC를 캐스팅, 플레이어를 Target으로 캐스팅)
  (bind _asbp_player (cast `/Game/PathfinderContent/Player/BP_Player` OtherActor))
  (cast `/Game/PathfinderContent/Monster/Boss/AIC_BossMonster` (`AIBlueprintHelperLibrary.GetAIController` self))
  (set `self.Player` _asbp_player))

(event `self.ReceiveAnyDamage`
  (params (Damage :type "Float (single-precision)") (DamageType :type "DamageType Object Reference") (InstigatedBy :type "Controller Object Reference") (DamageCauser :type "Actor Object Reference"))
  (bind (_returnvalue_x _returnvalue_y) (`KismetMathLibrary.BreakVector` (`SceneComponent.K2_GetComponentLocation` (`self.Mesh`))))
  (bind (_returnvalue_x_2 _returnvalue_y_2) (`KismetMathLibrary.BreakVector` (`SceneComponent.K2_GetComponentLocation` (`self.Mesh`))))
  ;[1 1 1] 피격과 사망
  (bind _output_get (set `self.IsHit` true))
  (`BlackboardComponent.SetValueAsBool` (`AIBlueprintHelperLibrary.GetBlackboard` null) (`self.IsHitBlackBoard`) _output_get)
  (set `self.Damage Causer` DamageCauser) ; 이 다음 피격 파티클 추가 예정
  (`NiagaraFunctionLibrary.SpawnSystemAtLocation` "/Game/PathfinderContent/Monster/Boss/HitImpact/NS_BossMonsterHitImpact.NS_BossMonsterHitImpact" (`KismetMathLibrary.MakeVector` _returnvalue_x_2 _returnvalue_y_2 -500.0))
  (bind _output_get_2 (`/Game/PathfinderContent/Component/BPC_StatSystem.DecreaseHealth` (`self.BPC_StatSystem`) Damage null (`self.Widget`)))
  (bind _output_get_3 (set `self.IsDead` _output_get_2))
  (if _output_get_3
    (`GameplayStatics.PlaySoundAtLocation` "/Game/PathfinderContent/Monster/Spider/Sound/SpiderDieSound.SpiderDieSound" (0.0 0.0 0.0) (struct) 1.0 1.0 0.0 null null null null)
    (`BlackboardComponent.SetValueAsBool` (`AIBlueprintHelperLibrary.GetBlackboard` null) (`self.IsHitBlackBoard`) (`self.IsDead`))
    (`NiagaraFunctionLibrary.SpawnSystemAtLocation` "/Game/PathfinderContent/Monster/Boss/HitImpact/NS_BossMonsterHitImpact.NS_BossMonsterHitImpact" (`KismetMathLibrary.MakeVector` _returnvalue_x _returnvalue_y -500.0) (struct) (10.0 1.0 10.0))
    (`self.K2_DestroyActor`) ; 액터 제거
    (else
      (bind _output_get_4 (set `self.IsHit` false)) ; 피격 애니메이션에 재생이 끝나면\nIsHit 값이 false가 되어\nBTT_AttackTask가 실행됨
      (`BlackboardComponent.SetValueAsBool` (`AIBlueprintHelperLibrary.GetBlackboard` null) (`self.IsHitBlackBoard`) _output_get_4))))

(fn `CreateBoiler`
  (bind _returnvalue (`|SpawnActorFromClass` "/Game/PathfinderContent/Monster/Boss/Pattern/Boiler/BP_Boiler.BP_Boiler_C" (`KismetMathLibrary.MakeTransform` (`SceneComponent.K2_GetComponentLocation` (`self.CapsuleComponent`)) (struct) (30.0 30.0 30.0)) "AlwaysSpawn" "MultiplyWithRoot" null null))
  (set `self.HeightDiff` (.z (- (- (`self.K2_GetActorLocation` (`self.PlayerCharacter`)) (* (`KismetMathLibrary.Normal` (- (`self.K2_GetActorLocation` (`self.PlayerCharacter`)) (`self.K2_GetActorLocation`))) (`self.Offset`))) (`self.K2_GetActorLocation`))))
  (set `self.Distance` (`KismetMathLibrary.VSize` (`KismetMathLibrary.MakeVector` (.x (- (- (`self.K2_GetActorLocation` (`self.PlayerCharacter`)) (* (`KismetMathLibrary.Normal` (- (`self.K2_GetActorLocation` (`self.PlayerCharacter`)) (`self.K2_GetActorLocation`))) (`self.Offset`))) (`self.K2_GetActorLocation`))) (.y (- (- (`self.K2_GetActorLocation` (`self.PlayerCharacter`)) (* (`KismetMathLibrary.Normal` (- (`self.K2_GetActorLocation` (`self.PlayerCharacter`)) (`self.K2_GetActorLocation`))) (`self.Offset`))) (`self.K2_GetActorLocation`))))))
  (set `self.V` (`KismetMathLibrary.Sqrt` (/ (* (`KismetMathLibrary.Square` (`self.Distance`)) (`self.G`)) (* (* (- (* (`self.Distance`) (`KismetMathLibrary.Tan` (`KismetMathLibrary.DegreesToRadians` (`self.LaunchAngle`)))) (`self.HeightDiff`)) 2.0) (`KismetMathLibrary.Square` (`KismetMathLibrary.Cos` (`KismetMathLibrary.DegreesToRadians` (`self.LaunchAngle`))))))))
  (`PrimitiveComponent.SetPhysicsLinearVelocity` (`/Game/PathfinderContent/Monster/Boss/Pattern/Boiler/BP_Boiler.CapsuleCollision` _returnvalue) (`KismetMathLibrary.MakeVector` (.x (* (* (`self.V`) (`KismetMathLibrary.Cos` (`KismetMathLibrary.DegreesToRadians` (`self.LaunchAngle`)))) (`KismetMathLibrary.Normal` (- (`self.K2_GetActorLocation` (`self.PlayerCharacter`)) (`self.K2_GetActorLocation`))))) (.y (* (* (`self.V`) (`KismetMathLibrary.Cos` (`KismetMathLibrary.DegreesToRadians` (`self.LaunchAngle`)))) (`KismetMathLibrary.Normal` (- (`self.K2_GetActorLocation` (`self.PlayerCharacter`)) (`self.K2_GetActorLocation`))))) (* (`KismetMathLibrary.Sin` (`KismetMathLibrary.DegreesToRadians` (`self.LaunchAngle`))) (`self.V`))) false "None")
  (`GameplayStatics.PlaySoundAtLocation` "/Game/PathfinderContent/Monster/Boss/Pattern/Boiler/boilerStart.boilerStart" (0.0 0.0 0.0) (struct) 1.0 1.0 0.0 null null null null))

(fn `CreateBox`
  (bind _returnvalue (`|SpawnActorFromClass` "/Game/PathfinderContent/Monster/Boss/Pattern/Box/BP_Box.BP_Box_C" (`KismetMathLibrary.MakeTransform` (`SceneComponent.K2_GetComponentLocation` (`self.CapsuleComponent`)) (struct) (30.0 30.0 30.0)) "AlwaysSpawn" "MultiplyWithRoot" null null))
  (`PrimitiveComponent.SetPhysicsLinearVelocity` (`/Game/PathfinderContent/Monster/Boss/Pattern/Box/BP_Box.BoxCollision` _returnvalue) (* (`KismetMathLibrary.Normal` (- (`self.K2_GetActorLocation` (`self.PlayerCharacter`)) (`self.K2_GetActorLocation`))) 4000.0) false "None")
  (`GameplayStatics.PlaySoundAtLocation` "/Game/PathfinderContent/Monster/Boss/Pattern/Box/bossBox.bossBox" (0.0 0.0 0.0) (struct) 1.0 1.0 0.0 null null null null))

(fn `CreateMini`
  (bind _returnvalue (`|SpawnActorFromClass` "/Game/PathfinderContent/Monster/Boss/Pattern/Mini/BP_MiniBossMonster.BP_MiniBossMonster_C" (`KismetMathLibrary.MakeTransform` (`SceneComponent.K2_GetComponentLocation` (`self.CapsuleComponent`)) (struct) (0.5 0.5 0.5)) "AdjustIfPossibleButAlwaysSpawn" "MultiplyWithRoot" null null))
  (set `self.HeightDiff` (.z (- (`self.K2_GetActorLocation` (`self.PlayerCharacter`)) (`self.K2_GetActorLocation`))))
  (set `self.Distance` (`KismetMathLibrary.VSize` (`KismetMathLibrary.MakeVector` (.x (- (`self.K2_GetActorLocation` (`self.PlayerCharacter`)) (`self.K2_GetActorLocation`))) (.y (- (`self.K2_GetActorLocation` (`self.PlayerCharacter`)) (`self.K2_GetActorLocation`))))))
  (set `self.V` (`KismetMathLibrary.Sqrt` (/ (* (`KismetMathLibrary.Square` (`self.Distance`)) (`self.G`)) (* (* (- (* (`self.Distance`) (`KismetMathLibrary.Tan` (`KismetMathLibrary.DegreesToRadians` (`self.LaunchAngle`)))) (`self.HeightDiff`)) 2.0) (`KismetMathLibrary.Square` (`KismetMathLibrary.Cos` (`KismetMathLibrary.DegreesToRadians` (`self.LaunchAngle`))))))))
  (`PrimitiveComponent.SetPhysicsLinearVelocity` (`Character.CapsuleComponent` _returnvalue) (`KismetMathLibrary.MakeVector` (.x (* (* (`self.V`) (`KismetMathLibrary.Cos` (`KismetMathLibrary.DegreesToRadians` (`self.LaunchAngle`)))) (`KismetMathLibrary.Normal` (- (`self.K2_GetActorLocation` (`self.PlayerCharacter`)) (`self.K2_GetActorLocation`))))) (.y (* (* (`self.V`) (`KismetMathLibrary.Cos` (`KismetMathLibrary.DegreesToRadians` (`self.LaunchAngle`)))) (`KismetMathLibrary.Normal` (- (`self.K2_GetActorLocation` (`self.PlayerCharacter`)) (`self.K2_GetActorLocation`))))) (* (`KismetMathLibrary.Sin` (`KismetMathLibrary.DegreesToRadians` (`self.LaunchAngle`))) (`self.V`))) false "None")
  (`GameplayStatics.PlaySoundAtLocation` "/Game/PathfinderContent/Monster/Boss/Pattern/Mini/orbStart.orbStart" (0.0 0.0 0.0) (struct) 1.0 1.0 0.0 null null null null))

(fn `UserConstructionScript`
  (`parent.UserConstructionScript`))