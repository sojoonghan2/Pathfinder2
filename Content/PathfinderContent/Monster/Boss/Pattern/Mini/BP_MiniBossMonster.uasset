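; Mini boss monster, under a boss pattern, that acts as a homing time bomb against the player.
; Once it drops below a fixed height, Tick switches off capsule physics, starts a sound and arms a fuse timer.
; It then faces and eases toward the player with VInterpTo until Boom stops movement, hides the mesh and spawns particles.
; Boom enables an overlap collider that damages the player once, and a second timer destroys the actor.
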(event `self.ReceiveBeginPlay`
  (`parent.ReceiveBeginPlay`)
  (`/Game/PathfinderContent/Component/BPC_StatSystem.InitializeEnemyState` (`self.BPC_StatSystem`) 100.0)
  (bind _asbp_player (cast `/Game/PathfinderContent/Player/BP_Player` (`GameplayStatics.GetPlayerCharacter` 0)))
  (set `self.PlayerCharacter` _asbp_player))

(event `self.ReceiveTick`
  (params (DeltaSeconds :type "Float (single-precision)"))
  (bind (_returnvalue_x _returnvalue_y _returnvalue_z) (`KismetMathLibrary.BreakVector` (`self.K2_GetActorLocation`)))
  (bind _returnvalue (`self.K2_GetActorLocation`))
  (bind _returnvalue_2 (`self.K2_GetActorLocation` (`self.PlayerCharacter`)))
  (if (not (`self.IsActive`))
    (if (<= _returnvalue_z -1400.0)
      (set `self.IsActive` true)
      (`PrimitiveComponent.SetSimulatePhysics` (`self.CapsuleComponent`) false)
      (bind _returnvalue_3 (`GameplayStatics.SpawnSoundAtLocation` "/Game/PathfinderContent/Monster/Boss/Pattern/Mini/orbMid.orbMid" (0.0 0.0 0.0) (struct) 1.0 1.0 0.0 null null))
      (set `self.MidSound` _returnvalue_3)
      (`KismetSystemLibrary.K2_SetTimer` null "Boom" 3.0))
    (else
      (`self.K2_SetActorRotation` (`KismetMathLibrary.FindLookAtRotation` _returnvalue _returnvalue_2)) ; 플레이어 쪽을 보도록
      (if (not (`self.IsBoom`))
        (`self.K2_SetActorLocation` (`KismetMathLibrary.VInterpTo` _returnvalue _returnvalue_2 DeltaSeconds 1.0))))))

(event `self.ExplosionCollision.OnComponentBeginOverlap`
  (params (OverlappedComponent :type "PrimitiveComponent Object Reference") (OtherActor :type "Actor Object Reference") (OtherComp :type "PrimitiveComponent Object Reference") (OtherBodyIndex :type Integer) (bFromSweep :type Boolean) (SweepResult :type "HitResult Structure (by ref)"))
  (bind _asbp_player (cast `/Game/PathfinderContent/Player/BP_Player` OtherActor))
  (`PrimitiveComponent.SetCollisionEnabled` (`self.ExplosionCollision`) "NoCollision")
  (`GameplayStatics.ApplyDamage` _asbp_player 15.0))

(fn `Boom`
  (bind _explosioncollision (`self.ExplosionCollision`))
  (set `self.IsBoom` true)
  (`GameplayStatics.PlaySoundAtLocation` "/Game/PathfinderContent/Monster/Boss/Pattern/Mini/orbEnd.orbEnd" (0.0 0.0 0.0) (struct) 1.0 1.0 0.0 null null null null)
  (`AudioComponent.Stop` (`self.MidSound`))
  (`AddComponent|NODE_AddParticleSystemComponent-0` :`RelativeTransform` (`KismetMathLibrary.MakeTransform` (0.0 0.0 -100.0) (struct) (10.0 10.0 10.0)))
  (`KismetSystemLibrary.K2_SetTimer` null "Destroy" 2.0)
  (`SceneComponent.SetVisibility` (`self.Mesh`) false false)
  (`PrimitiveComponent.SetCollisionEnabled` _explosioncollision "QueryAndPhysics")
  (`PrimitiveComponent.SetCollisionResponseToChannel` _explosioncollision "ECC_Pawn" "ECR_Overlap"))

(fn `Destroy`
  (`self.K2_DestroyActor`))

(fn `UserConstructionScript`
  (`parent.UserConstructionScript`))