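; BP_DarkBead is a projectile, filed under boss patterns, that triggers a dark effect on the player.
; On BeginPlay it locks a direction toward the player's current position and sets a three-second lifespan.
; Tick moves it along that fixed line with a swept world offset, without homing.
; Overlapping the player calls StartDark on BP_Player; the bead is not destroyed on contact.
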(event `self.ReceiveBeginPlay`
  (bind _asbp_player (cast `/Game/PathfinderContent/Player/BP_Player` (`GameplayStatics.GetPlayerCharacter` 0)))
  (bind _output_get (set `self.Player Character` _asbp_player))
  (set `self.PlayerLocation` (`self.K2_GetActorLocation` _output_get))
  (set `self.MoveLocation` (`KismetMathLibrary.Normal` (- (`self.PlayerLocation`) (`self.K2_GetActorLocation`))))
  (`self.SetLifeSpan` 3.0))

(event `self.ReceiveTick`
  (params (DeltaSeconds :type "Float (single-precision)"))
  (`/Engine/EditorBlueprintResources/StandardMacros.IsValid` (`self.Player Character`)
    (:`Is Valid`
      (`self.K2_AddActorWorldOffset` (* (`self.MoveLocation`) DeltaSeconds 3000.0) true))))

(event `self.Collision.OnComponentBeginOverlap`
  (params (OverlappedComponent :type "PrimitiveComponent Object Reference") (OtherActor :type "Actor Object Reference") (OtherComp :type "PrimitiveComponent Object Reference") (OtherBodyIndex :type Integer) (bFromSweep :type Boolean) (SweepResult :type "HitResult Structure (by ref)"))
  (bind _asbp_player (cast `/Game/PathfinderContent/Player/BP_Player` OtherActor))
  (`/Game/PathfinderContent/Player/BP_Player.StartDark` _asbp_player))

(fn `UserConstructionScript`)