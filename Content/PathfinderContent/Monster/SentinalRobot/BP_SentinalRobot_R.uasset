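; Sentinel Robot enemy that melee-attacks the player and resists damage while its own BP_Core survives.
; BeginPlay spawns that core at one of two fixed spots, depending on whether another core exists.
; AI overlap passes the player to its AI controller, while StartAttack/StopAttack control timed forearm sphere traces damaging Player-tagged actors.
; Incoming damage is cut tenfold while the core lives, feeds BPCStatSystem and the hit blackboard key, and destroys the robot on death.
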(event `self.ReceiveBeginPlay`
  ; Initialize
  (`parent.ReceiveBeginPlay`)
  (`/Game/PathfinderContent/Component/BPC_StatSystem.InitializeEnemyState` (`self.BPC_StatSystem`) 300.0)
  (bind _returnvalue (`GameplayStatics.GetActorOfClass` "/Game/PathfinderContent/Monster/SentinalRobot/Core/BP_Core.BP_Core_C"))
  (`/Engine/EditorBlueprintResources/StandardMacros.IsValid` _returnvalue
    (:`Is Valid`
      (bind _returnvalue_2 (`|SpawnActorFromClass` "/Game/PathfinderContent/Monster/SentinalRobot/Core/BP_Core.BP_Core_C" (`KismetMathLibrary.MakeTransform` (-3000.0 -902.368085 400.0)) "AlwaysSpawn" "MultiplyWithRoot" null null)) ; 본인 코어 생성
      (set `self.Core` _returnvalue_2))
    (:`Is Not Valid`
      (bind _returnvalue_3 (`|SpawnActorFromClass` "/Game/PathfinderContent/Monster/SentinalRobot/Core/BP_Core.BP_Core_C" (`KismetMathLibrary.MakeTransform` (3000.0 1211.789943 400.0)) "AlwaysSpawn" "MultiplyWithRoot" null null)) ; 본인 코어 생성
      (set `self.Core` _returnvalue_3))))

(event `self.AICollision.OnComponentBeginOverlap`
  (params (OverlappedComponent :type "PrimitiveComponent Object Reference") (OtherActor :type "Actor Object Reference") (OtherComp :type "PrimitiveComponent Object Reference") (OtherBodyIndex :type Integer) (bFromSweep :type Boolean) (SweepResult :type "HitResult Structure (by ref)"))
  ;[1 1 1] AI의 플레이어 감지(플레이어와 AIC를 캐스팅, 플레이어를 Target으로 캐스팅)
  (bind _asbp_player (cast `/Game/PathfinderContent/Player/BP_Player` OtherActor))
  (bind _asaic_sentinal_robot (cast `/Game/PathfinderContent/Monster/SentinalRobot/AIC_SentinalRobot` (`AIBlueprintHelperLibrary.GetAIController` self)))
  (`/Game/PathfinderContent/Monster/SentinalRobot/AIC_SentinalRobot.SetTarget` _asaic_sentinal_robot _asbp_player)
  (set `self.Player` _asbp_player))

(event `StartAttack`
  ;[1 1 1] AttackTrace
  (bind _returnvalue (`KismetSystemLibrary.K2_SetTimerDelegate` (delegate `Attack`) 0.01)) ; 일정 시간마다 지정한 이벤트를 반복
  (set `self.AttackTimerHander` _returnvalue) ; Set Timer by Event의 Time을\nAttack Timer Hander 타이머에 저장
)

(event `Attack`
  ;[1 1 1] AttackTrace
  (bind (_outhit _returnvalue) (`KismetSystemLibrary.SphereTraceSingle` :`Start` (`SceneComponent.K2_GetComponentLocation` (`self.HandStart`)) :`End` (`SceneComponent.K2_GetComponentLocation` (`self.HandEnd`)) :`Radius` 120.0 :`TraceChannel` "TraceTypeQuery1" :`DrawDebugType` "ForDuration"))
  (if _returnvalue
    (bind (_bblockinghit _binitialoverlap _time _distance _location _impactpoint _normal _impactnormal _physmat _hitactor) (`GameplayStatics.BreakHitResult` _outhit))
    (if (`self.ActorHasTag` _hitactor "Player")
      (`GameplayStatics.ApplyDamage` _hitactor 20.0 null self))))

(event `StopAttack`
  ;[1 1 1] AttackTrace
  (`KismetSystemLibrary.K2_ClearAndInvalidateTimerHandle` (`self.AttackTimerHander`)) ; 공격이 끝나면 Attack Timer를 끔
)

(event `self.ReceiveAnyDamage`
  (params (Damage :type "Float (single-precision)") (DamageType :type "DamageType Object Reference") (InstigatedBy :type "Controller Object Reference") (DamageCauser :type "Actor Object Reference"))
  ;[1 1 1] 피격과 사망
  (set `self.Damage` Damage)
  (`/Engine/EditorBlueprintResources/StandardMacros.IsValid` (`self.Core`) ; 코어가 부숴지지 않았으면
    (:`Is Valid`
      (bind _output_get (set `self.Damage` (/ (`self.Damage`) 10.0))))
    (:`Is Not Valid`
      _))
  (bind _output_get_2 (set `self.IsHit` true))
  (`BlackboardComponent.SetValueAsBool` (`AIBlueprintHelperLibrary.GetBlackboard` null) (`self.IsHitBlackBoard`) _output_get_2)
  (set `self.Damage Causer` DamageCauser) ; 이 다음 피격 파티클 추가 예정
  (`NiagaraFunctionLibrary.SpawnSystemAtLocation` "/Game/PathfinderContent/Monster/SentinalRobot/HitImpact/NS_SentinalRobotHitImpact.NS_SentinalRobotHitImpact" (`self.HitLocation`))
  (bind _output_get_3 (`/Game/PathfinderContent/Component/BPC_StatSystem.DecreaseHealth` (`self.BPC_StatSystem`) _output_get null (`self.Widget`)))
  (bind _output_get_4 (set `self.IsDead` _output_get_3))
  (if _output_get_4
    (`GameplayStatics.PlaySoundAtLocation` "/Game/PathfinderContent/Monster/SentinalRobot/Sound/factoryMonsterDie.factoryMonsterDie" (0.0 0.0 0.0) (struct) 1.0 1.0 0.0 null null null null)
    (`BlackboardComponent.SetValueAsBool` (`AIBlueprintHelperLibrary.GetBlackboard` null) (`self.IsHitBlackBoard`) (`self.IsDead`))
    (`self.K2_DestroyActor`) ; 액터 제거
    (else
      (bind _output_get_5 (set `self.IsHit` false)) ; 피격 애니메이션에 재생이 끝나면\nIsHit 값이 false가 되어\nBTT_AttackTask가 실행됨
      (`BlackboardComponent.SetValueAsBool` (`AIBlueprintHelperLibrary.GetBlackboard` null) (`self.IsHitBlackBoard`) _output_get_5))))

(fn `UserConstructionScript`
  (`parent.UserConstructionScript`)
  (`SceneComponent.K2_AttachToComponent` (`self.HandStart`) (`self.Mesh`) "Bip001_L_Forearm" "KeepRelative" "KeepRelative" "KeepRelative" true)
  (`SceneComponent.K2_AttachToComponent` (`self.HandEnd`) (`self.Mesh`) "Bip001_L_Forearm" "KeepRelative" "KeepRelative" "KeepRelative" true))