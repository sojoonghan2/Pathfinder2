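; BP_Core is a damageable, spinning core actor filed under the SentinalRobot monster.
; A stat component initializes it with enemy state on BeginPlay, and Tick rotates it around yaw at a steady, delta-time-scaled rate.
; Any damage spawns a Niagara impact at the hit location and reduces health through the stat component, which also receives the monster widget.
; The actor is destroyed when that call reports death.
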(event `self.ReceiveBeginPlay`
  ; Initialize
  (`parent.ReceiveBeginPlay`)
  (`/Game/PathfinderContent/Component/BPC_StatSystem.InitializeEnemyState` (`self.BPC_StatSystem`) 100.0))

(event `self.ReceiveAnyDamage`
  (params (Damage :type "Float (single-precision)") (DamageType :type "DamageType Object Reference") (InstigatedBy :type "Controller Object Reference") (DamageCauser :type "Actor Object Reference"))
  ;[1 1 1] 피격과 사망
  (set `self.IsHit` true)
  (set `self.Damage Causer` DamageCauser) ; 이 다음 피격 파티클 추가 예정
  (`NiagaraFunctionLibrary.SpawnSystemAtLocation` "/Game/PathfinderContent/Monster/SentinalRobot/Core/HitImpact/NS_CoreHitImpact.NS_CoreHitImpact" (`self.HitLocation`))
  (bind _output_get (`/Game/PathfinderContent/Component/BPC_StatSystem.DecreaseHealth` (`self.BPC_StatSystem`) Damage null (`self.Widget`)))
  (bind _output_get_2 (set `self.IsDead` _output_get))
  (if _output_get_2
    (`self.K2_DestroyActor`)
    (else
      (set `self.IsHit` false))))

(event `self.ReceiveTick`
  (params (DeltaSeconds :type "Float (single-precision)"))
  (bind (_returnvalue_roll _returnvalue_pitch _returnvalue_yaw) (`KismetMathLibrary.BreakRotator` (`self.K2_GetActorRotation`)))
  ; Tick
  (`parent.ReceiveTick` 0.0)
  (`self.K2_SetActorRotation` (`KismetMathLibrary.MakeRotator` _returnvalue_roll _returnvalue_pitch (+ (* DeltaSeconds 100.0) _returnvalue_yaw))))

(fn `UserConstructionScript`
  (`parent.UserConstructionScript`))