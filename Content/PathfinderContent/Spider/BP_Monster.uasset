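; BP_Monster is a spider enemy that deals melee damage and can be hurt and killed.
; StartAttack runs a fast timer that sphere-traces between two hand points and damages Player-tagged actors until StopAttack clears it.
; Incoming damage spawns blood, lowers health through BPCStatSystem and writes hit state to the Blackboard; death plays a sound and destroys the actor.
; RotateToAttackActor yaws it toward a given actor.
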(event `StartAttack`
  ;[1 1 1] AttackTrace
  (bind _returnvalue (`KismetSystemLibrary.K2_SetTimerDelegate` (delegate `Attack`) 0.01)) ; 일정 시간마다 지정한 이벤트를 반복
  (set `self.AttackTimerHander` _returnvalue) ; Set Timer by Event의 Time을\nAttack Timer Hander 타이머에 저장
)

(event `Attack`
  ;[1 1 1] AttackTrace
  (bind (_outhit _returnvalue) (`KismetSystemLibrary.SphereTraceSingle` :`Start` (`SceneComponent.K2_GetComponentLocation` (`self.HandStart`)) :`End` (`SceneComponent.K2_GetComponentLocation` (`self.HandEnd`)) :`Radius` 50.0 :`TraceChannel` "TraceTypeQuery1" :`DrawDebugType` "ForDuration"))
  (if _returnvalue
    (bind (_bblockinghit _binitialoverlap _time _distance _location _impactpoint _normal _impactnormal _physmat _hitactor) (`GameplayStatics.BreakHitResult` _outhit))
    (if (`self.ActorHasTag` _hitactor "Player")
      (`GameplayStatics.ApplyDamage` _hitactor 20.0 null self))))

(event `StopAttack`
  ;[1 1 1] AttackTrace
  (`KismetSystemLibrary.K2_ClearAndInvalidateTimerHandle` (`self.AttackTimerHander`)) ; 공격이 끝나면 Attack Timer를 끔
)

(event `self.ReceiveAnyDamage`
  (params (Damage :type "Float (single-precision)") (DamageType :type "DamageType Object Reference") (InstigatedBy :type "Controller Object Reference") (DamageCauser :type "Actor Object Reference"))
  ;[1 1 1] 피격과 사망
  (bind _output_get (set `self.IsHit` true))
  (`BlackboardComponent.SetValueAsBool` (`AIBlueprintHelperLibrary.GetBlackboard` null) (`self.IsHitBlackBoard`) _output_get)
  (set `self.Damage Causer` DamageCauser) ; 이 다음 피격 파티클 추가 예정
  (`NiagaraFunctionLibrary.SpawnSystemAtLocation` "/Game/PathfinderContent/Spider/HitImpact/NS_HitBlood.NS_HitBlood" (`self.HitLocation`))
  (bind _output_get_2 (`/Game/PathfinderContent/Component/BPC_StatSystem.DecreaseHealth` (`self.BPC_StatSystem`) Damage null (`self.Widget`)))
  (bind _output_get_3 (set `self.IsDead` _output_get_2))
  (if _output_get_3
    (`GameplayStatics.PlaySoundAtLocation` "/Game/PathfinderContent/Spider/Sound/SpiderDieSound.SpiderDieSound" (0.0 0.0 0.0) (struct) 1.0 1.0 0.0 null null null null)
    (`BlackboardComponent.SetValueAsBool` (`AIBlueprintHelperLibrary.GetBlackboard` null) (`self.IsHitBlackBoard`) (`self.IsDead`))
    (`NiagaraFunctionLibrary.SpawnSystemAtLocation` "/Game/PathfinderContent/Spider/HitImpact/NS_HitBlood.NS_HitBlood" (`self.HitLocation`) (struct) (10.0 1.0 10.0))
    (`self.K2_DestroyActor`) ; 액터 제거
    (else
      (bind _output_get_4 (set `self.IsHit` false)) ; 피격 애니메이션에 재생이 끝나면\nIsHit 값이 false가 되어\nBTT_AttackTask가 실행됨
      (`BlackboardComponent.SetValueAsBool` (`AIBlueprintHelperLibrary.GetBlackboard` null) (`self.IsHitBlackBoard`) _output_get_4))))

(fn `RotateToAttackActor`
  (params (AttackActor :type "Actor Object Reference"))
  (bind (_returnvalue_roll _returnvalue_pitch _returnvalue_yaw) (`KismetMathLibrary.BreakRotator` (`KismetMathLibrary.FindLookAtRotation` (`self.K2_GetActorLocation`) (`self.K2_GetActorLocation` AttackActor))))
  (`self.K2_SetActorRotation` (`KismetMathLibrary.MakeRotator` 0.0 0.0 _returnvalue_yaw)))

(fn `UserConstructionScript`)