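; Enemy Sentinal robot that is driven by an AI controller and blackboard, detects the player, and takes damage.
; Sphere overlap with BP_Player sets that player as the target on AIC_SentinalRobot.
; AnyDamage spawns blood VFX, decreases health through BPCStatSystem, and pulses the hit blackboard bool, clearing it immediately if the robot survives.
; On death it writes true to that same hit key, plays a sound and larger VFX, then destroys itself.
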(event `self.Sphere.OnComponentBeginOverlap`
  (params (OverlappedComponent :type "PrimitiveComponent Object Reference") (OtherActor :type "Actor Object Reference") (OtherComp :type "PrimitiveComponent Object Reference") (OtherBodyIndex :type Integer) (bFromSweep :type Boolean) (SweepResult :type "HitResult Structure (by ref)"))
  ;[1 1 1] AI의 플레이어 감지(플레이어와 AIC를 캐스팅, 플레이어를 Target으로 캐스팅)
  (bind _asbp_player (cast `/Game/PathfinderContent/Player/BP_Player` OtherActor))
  (bind _asaic_sentinal_robot (cast `/Game/PathfinderContent/SentinalRobot/AIC_SentinalRobot` (`AIBlueprintHelperLibrary.GetAIController` self)))
  (`/Game/PathfinderContent/SentinalRobot/AIC_SentinalRobot.SetTarget` _asaic_sentinal_robot _asbp_player)
  (set `self.Player` _asbp_player))

(event `self.ReceiveAnyDamage`
  (params (Damage :type "Float (single-precision)") (DamageType :type "DamageType Object Reference") (InstigatedBy :type "Controller Object Reference") (DamageCauser :type "Actor Object Reference"))
  ;[1 1 1] 피격과 사망(동작 안하는 이유를 파악해야 함)
  (bind _output_get (set `self.IsHit` true))
  (`BlackboardComponent.SetValueAsBool` (`AIBlueprintHelperLibrary.GetBlackboard` null) (`self.IsHitBlackBoard`) _output_get)
  (set `self.Damage Causer` DamageCauser) ; 이 다음 피격 파티클 추가 예정
  (`NiagaraFunctionLibrary.SpawnSystemAtLocation` "/Game/PathfinderContent/Spider/HitImpact/NS_HitBlood.NS_HitBlood" (`self.HitLocation`))
  (bind _output_get_2 (`/Game/PathfinderContent/Component/BPC_StatSystem.DecreaseHealth` (`self.BPC_StatSystem`) Damage null (`self.Widget`)))
  (bind _output_get_3 (set `self.IsDead` _output_get_2))
  (if _output_get_3
    (`GameplayStatics.PlaySoundAtLocation` "/Game/PathfinderContent/SentinalRobot/Sound/factoryMonsterDie.factoryMonsterDie" (0.0 0.0 0.0) (struct) 1.0 1.0 0.0 null null null null)
    (`BlackboardComponent.SetValueAsBool` (`AIBlueprintHelperLibrary.GetBlackboard` null) (`self.IsHitBlackBoard`) (`self.IsDead`))
    (`NiagaraFunctionLibrary.SpawnSystemAtLocation` "/Game/PathfinderContent/Spider/HitImpact/NS_HitBlood.NS_HitBlood" (`self.HitLocation`) (struct) (10.0 1.0 10.0))
    (`self.K2_DestroyActor`) ; 액터 제거
    (else
      (bind _output_get_4 (set `self.IsHit` false)) ; 피격 애니메이션에 재생이 끝나면\nIsHit 값이 false가 되어\nBTT_AttackTask가 실행됨
      (`BlackboardComponent.SetValueAsBool` (`AIBlueprintHelperLibrary.GetBlackboard` null) (`self.IsHitBlackBoard`) _output_get_4))))

(fn `UserConstructionScript`
  (`parent.UserConstructionScript`))