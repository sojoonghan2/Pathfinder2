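; BP_SentinalRobot_R is a sentinel robot enemy that detects the player by proximity and hands it to its AI controller.
; On BeginPlay it calls the parent and initializes its enemy state through BPCStatSystem.
; When BP_Player enters the detection Sphere, it sets that player as AIC_SentinalRobot's target and then caches the reference.
; Tick and actor overlap events are disabled stubs.
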(event `self.ReceiveBeginPlay`
  (`parent.ReceiveBeginPlay`)
  (`/Game/PathfinderContent/Component/BPC_StatSystem.InitializeEnemyState` (`self.BPC_StatSystem`) 300.0))

(event `self.Sphere.OnComponentBeginOverlap`
  (params (OverlappedComponent :type "PrimitiveComponent Object Reference") (OtherActor :type "Actor Object Reference") (OtherComp :type "PrimitiveComponent Object Reference") (OtherBodyIndex :type Integer) (bFromSweep :type Boolean) (SweepResult :type "HitResult Structure (by ref)"))
  ;[1 1 1] AI의 플레이어 감지(플레이어와 AIC를 캐스팅, 플레이어를 Target으로 캐스팅)
  (bind _asbp_player (cast `/Game/PathfinderContent/Player/BP_Player` OtherActor))
  (bind _asaic_sentinal_robot (cast `/Game/PathfinderContent/SentinalRobot/AIC_SentinalRobot` (`AIBlueprintHelperLibrary.GetAIController` self)))
  (`/Game/PathfinderContent/SentinalRobot/AIC_SentinalRobot.SetTarget` _asaic_sentinal_robot _asbp_player)
  (set `self.Player` _asbp_player))

(fn `UserConstructionScript`
  (`parent.UserConstructionScript`))