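; Actor component that tracks an ammo count and reports it to the player HUD.
; On BeginPlay it takes the first top-level WB_HUD widget and fills current ammo to the maximum.
; DecreaseAmmo removes one round while any remain, using a HUD reference passed in by the caller.
; Both functions push current and max ammo to the HUD's percent message directly.
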(event `self.ReceiveBeginPlay`
  (bind _foundwidgets (`WidgetBlueprintLibrary.GetAllWidgetsOfClass` "/Game/PathfinderContent/UI/WB_HUD.WB_HUD_C"))
  (`self.InitializeAmmo` (`|GetArrayItem` _foundwidgets)))

(fn `DecreaseAmmo`
  (params (PlayerHUD :type "/Game/PathfinderContent/UI/WB_HUD Object Reference"))
  (returns (CurrentAmmo :type "Float (double-precision)"))
  (if (> (`self.CurrentAmmo`) 0.0)
    (set `self.CurrentAmmo` (- (`self.CurrentAmmo`) 1.0))
    (message `/Game/PathfinderContent/Interfaces/BPI_Ammo.SetAmmoPercent` (`local.PlayerHUD`) (`self.MaxAmmo`) (`self.CurrentAmmo`))
    (return (`self.CurrentAmmo`))))

(fn `InitializeAmmo`
  (params (PlayerHUD :type "/Game/PathfinderContent/UI/WB_HUD Object Reference"))
  (returns (CurrentAmmo :type "Float (double-precision)"))
  (set `self.CurrentAmmo` (`self.MaxAmmo`))
  (message `/Game/PathfinderContent/Interfaces/BPI_Ammo.SetAmmoPercent` (`local.PlayerHUD`) (`self.MaxAmmo`) (`self.CurrentAmmo`))
  (return (`self.CurrentAmmo`)))