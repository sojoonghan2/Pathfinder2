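; Attack component for the Murdock player character that handles aimed zoom and hitscan shooting.
; Enhanced Input aiming toggles camera zoom, crosshair visibility and orient-rotation-to-movement.
; The Fire event works only while aiming, playing muzzle flash, sound and montage.
; It traces from the camera to find the aim point, then from the muzzle toward it to apply damage, with debug lines drawn.
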(event `self.ReceiveBeginPlay`
  ; Player Casting
  (bind _asbp_murdock (cast `/Game/PathfinderContent/Player/Murdock/BP_Murdock` (`GameplayStatics.GetPlayerCharacter` 0)))
  (set `self.PlayerCharacter` _asbp_murdock))

(event `EnhancedInput|/Game/PathfinderContent/Player/Murdock/Input/IA_Aiming`
  (params (ActionValue :type Boolean) (ElapsedSeconds :type "Float (double-precision)") (TriggeredSeconds :type "Float (double-precision)") (InputAction :type "InputAction Object Reference" :default "/Game/PathfinderContent/Player/Murdock/Input/IA_Aiming.IA_Aiming"))
  ; Zoom
  (:`Triggered`
    (set `self.IsAiming` true)
    (set `CharacterMovementComponent.bOrientRotationToMovement` false (`Character.CharacterMovement` (`self.PlayerCharacter`)))
    (`/Game/PathfinderContent/Player/Murdock/BP_Murdock.ZoomByAiming` (`self.PlayerCharacter`))
    (`Widget.SetVisibility` (`/Game/PathfinderContent/UI/WB_HUD.Crosshair` (`/Game/PathfinderContent/Player/Murdock/BP_MurdockController.PlayerHUD` (`/Game/PathfinderContent/Player/Murdock/BP_Murdock.PlayerController` (`self.PlayerCharacter`)))) "Visible"))
  (:`Canceled`
    (set `self.IsAiming` false :!label _label)
    (set `CharacterMovementComponent.bOrientRotationToMovement` true (`Character.CharacterMovement` (`self.PlayerCharacter`)))
    (`/Game/PathfinderContent/Player/Murdock/BP_Murdock.ZoomOutByAimingEnd` (`self.PlayerCharacter`))
    (`Widget.SetVisibility` (`/Game/PathfinderContent/UI/WB_HUD.Crosshair` (`/Game/PathfinderContent/Player/Murdock/BP_MurdockController.PlayerHUD` (`/Game/PathfinderContent/Player/Murdock/BP_Murdock.PlayerController` (`self.PlayerCharacter`)))) "Hidden"))
  (:`Completed`
    (goto _label)))

(event `Fire`
  (bind _camera (`/Game/PathfinderContent/Player/Murdock/BP_Murdock.Camera` (`self.PlayerCharacter`)))
  (bind _returnvalue (`SceneComponent.K2_GetComponentLocation` (`/Game/PathfinderContent/Player/Murdock/BP_Murdock.Muzzle` (`self.PlayerCharacter`))))
  (bind _returnvalue_2 (`SceneComponent.K2_GetComponentLocation` _camera))
  (bind _returnvalue_3 (* (`SceneComponent.GetForwardVector` _camera) 20000.0))
  ; Fire
  (if (`self.IsAiming`)
    (`self.PlayMuzzleFlash`)
    (if (> (`KismetMathLibrary.VSize` (`MovementComponent.Velocity` (`Character.CharacterMovement` (`self.PlayerCharacter`)))) 0.0)
      (`|PlayMontage` (`Character.Mesh` (`self.PlayerCharacter`)) "/Game/PathfinderContent/Player/Murdock/Animation/Fire_Fast_Montage.Fire_Fast_Montage" ; 움직이면서 쏘도록 변경해야 함
        (:`then`
          _))
      (else
        (`|PlayMontage` (`Character.Mesh` (`self.PlayerCharacter`)) "/Game/PathfinderContent/Player/Murdock/Animation/Fire_Fast_Montage.Fire_Fast_Montage"
          (:`then`
            _))))
    (bind (_outhit _returnvalue_4) (`KismetSystemLibrary.LineTraceSingle` :`Start` _returnvalue_2 :`End` (+ _returnvalue_2 _returnvalue_3) :`TraceChannel` "TraceTypeQuery1" :`DrawDebugType` "ForDuration"))
    (if _returnvalue_4
      (bind (_outhit_2 _returnvalue_5) (`KismetSystemLibrary.LineTraceSingle` :`Start` _returnvalue :`End` (* (`KismetMathLibrary.Normal` (- (`.ImpactPoint` (`GameplayStatics.BreakHitResult` _outhit)) _returnvalue)) 20000.0) :`TraceChannel` "TraceTypeQuery1" :`DrawDebugType` "ForDuration"))
      (if _returnvalue_5
        (`GameplayStatics.ApplyDamage` (`.HitActor` (`GameplayStatics.BreakHitResult` _outhit_2)) 33.0 null (`self.PlayerCharacter`)))
      (else
        (`KismetSystemLibrary.LineTraceSingle` :`Start` _returnvalue :`End` (+ _returnvalue _returnvalue_3) :`TraceChannel` "TraceTypeQuery1" :`DrawDebugType` "ForDuration")))))

(fn `PlayMuzzleFlash`
  (`NiagaraFunctionLibrary.SpawnSystemAtLocation` "/Game/PathfinderContent/Player/MuzzleFlash/MuzzleFlash/Niagara/NS_MuzzleFlash.NS_MuzzleFlash" (`SceneComponent.K2_GetComponentLocation` (`/Game/PathfinderContent/Player/Murdock/BP_Murdock.Muzzle` (`self.PlayerCharacter`))) (`KismetMathLibrary.ComposeRotators` (`KismetMathLibrary.MakeRotFromX` (`Actor.GetActorForwardVector` (`self.PlayerCharacter`))) (`KismetMathLibrary.MakeRotator` 0.0 0.0 -90.0)) (1.0 1.0 1.0) false)
  (`GameplayStatics.PlaySoundAtLocation` "/Game/PathfinderContent/Player/Murdock/Sound/shoot.shoot" (0.0 0.0 0.0) (struct) 1.0 1.0 0.0 null null null null))