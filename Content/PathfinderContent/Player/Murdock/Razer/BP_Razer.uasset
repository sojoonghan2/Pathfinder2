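; BP_Razer is a short-lived beam actor for Murdock's Razer skill that damages what its collision overlaps.
; On BeginPlay it caches the player, deactivates the PElevenBeam particle after a brief GPU initialization delay, then destroys itself shortly afterward.
; Overlaps skip components tagged AICollision and apply damage read from the Murdock skill data table, with the player as damage causer.
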(event `self.ReceiveBeginPlay`
  (bind _asbp_player (cast `/Game/PathfinderContent/Player/BP_Player` (`GameplayStatics.GetPlayerCharacter` 0)))
  (set `self.PlayerCharacter` _asbp_player)
  (`KismetSystemLibrary.Delay` 0.1) ; GPU를 위한 파티클 컴포넌트 초기화 대기 프레임
  (`ActorComponent.SetActive` (`self.P_ElevenBeam`) false false)
  (`KismetSystemLibrary.Delay` 1.5)
  (`self.K2_DestroyActor`))

(event `self.Collision.OnComponentBeginOverlap`
  (params (OverlappedComponent :type "PrimitiveComponent Object Reference") (OtherActor :type "Actor Object Reference") (OtherComp :type "PrimitiveComponent Object Reference") (OtherBodyIndex :type Integer) (bFromSweep :type Boolean) (SweepResult :type "HitResult Structure (by ref)"))
  (if (not (`ActorComponent.ComponentHasTag` OtherComp "AICollision"))
    (bind _returnvalue (`|GetDataTableRow` "/Game/PathfinderContent/Player/Murdock/DT_MurdockSkillInformation.DT_MurdockSkillInformation" "Razer")
      (:`then`
        (`GameplayStatics.ApplyDamage` OtherActor (`.SkillDamage_8_B7C91E384BC8535F3922369F075CA282` (break `/Game/PathfinderContent/Player/Murdock/S_SkillInformation` _returnvalue)) null (`self.PlayerCharacter`))))))

(fn `UserConstructionScript`)