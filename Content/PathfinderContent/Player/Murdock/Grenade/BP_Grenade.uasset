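; BP_Grenade is Murdock's grenade skill actor, which explodes on impact and damages actors in its blast volume.
; A collision hit activates the explosion effect, hides the mesh and enables the explosion collision, then destroys the actor after a short delay.
; Each actor that begins overlapping the explosion collision takes damage read from the Grenade row of the Murdock skill data table.
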(event `self.Collision.OnComponentHit`
  (params (HitComponent :type "PrimitiveComponent Object Reference") (OtherActor :type "Actor Object Reference") (OtherComp :type "PrimitiveComponent Object Reference") (NormalImpulse :type "Vector Structure") (Hit :type "HitResult Structure (by ref)"))
  (`ActorComponent.SetActive` (`self.NS_Explosion`) true false)
  (`SceneComponent.SetVisibility` (`self.StaticMesh`) false false)
  (`PrimitiveComponent.SetCollisionEnabled` (`self.ExplosionCollision`) "QueryAndPhysics")
  (`KismetSystemLibrary.Delay` 2.0)
  (`self.K2_DestroyActor`))

(event `self.ExplosionCollision.OnComponentBeginOverlap`
  (params (OverlappedComponent :type "PrimitiveComponent Object Reference") (OtherActor :type "Actor Object Reference") (OtherComp :type "PrimitiveComponent Object Reference") (OtherBodyIndex :type Integer) (bFromSweep :type Boolean) (SweepResult :type "HitResult Structure (by ref)"))
  (bind _returnvalue (`|GetDataTableRow` "/Game/PathfinderContent/Player/Murdock/DT_MurdockSkillInformation.DT_MurdockSkillInformation" "Grenade")
    (:`then`
      (`GameplayStatics.ApplyDamage` OtherActor (`.SkillDamage_8_B7C91E384BC8535F3922369F075CA282` (break `/Game/PathfinderContent/Player/Murdock/S_SkillInformation` _returnvalue))))))

(fn `UserConstructionScript`)