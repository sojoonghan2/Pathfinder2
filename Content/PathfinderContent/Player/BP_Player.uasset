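; Player character Blueprint for Murdock, handling Enhanced Input movement, look, sprint, reload and dash.
; Damage goes through BPCStatSystem to play a hit reaction or death and destroy, with flags blocking movement; reload is delegated to BPCAttackSystem.
; Dash is a timeline-driven swept offset with Niagara and sound, its data-table cooldown counted down on Tick and sent to the HUD.
; Aim zoom events play or reverse a spring-arm and camera timeline.
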(event `self.ReceiveBeginPlay`
  ; PlayerController 매핑
  (bind _asbp_murdock_controller (cast `/Game/PathfinderContent/Player/Murdock/BP_MurdockController` (`self.GetController`)))
  (bind _output_get (set `self.PlayerController` _asbp_murdock_controller))
  (message `EnhancedInputSubsystemInterface.AddMappingContext` (pcsubsystem `EnhancedInputLocalPlayerSubsystem` _output_get) "/Game/PathfinderContent/Player/Murdock/Input/IMC_Murdock.IMC_Murdock" 0 (struct)))

(event `EnhancedInput|/Game/PathfinderContent/Player/Murdock/Input/IA_LookAround`
  (params (ActionValue :type "Vector2D Structure") (ElapsedSeconds :type "Float (double-precision)") (TriggeredSeconds :type "Float (double-precision)") (InputAction :type "InputAction Object Reference" :default "/Game/PathfinderContent/Player/Murdock/Input/IA_LookAround.IA_LookAround"))
  ; IA_LookAround
  (:`Triggered`
    (`self.AddControllerYawInput` ActionValue_X)
    (`self.AddControllerPitchInput` (* ActionValue_Y -1.0))))

(event `EnhancedInput|/Game/PathfinderContent/Player/Murdock/Input/IA_Movement`
  (params (ActionValue :type "Vector2D Structure") (ElapsedSeconds :type "Float (double-precision)") (TriggeredSeconds :type "Float (double-precision)") (InputAction :type "InputAction Object Reference" :default "/Game/PathfinderContent/Player/Murdock/Input/IA_Movement.IA_Movement"))
  (bind (_returnvalue_roll _returnvalue_pitch _returnvalue_yaw) (`KismetMathLibrary.BreakRotator` (`self.GetControlRotation`)))
  (bind (_returnvalue_roll_2 _returnvalue_pitch_2 _returnvalue_yaw_2) (`KismetMathLibrary.BreakRotator` (`self.GetControlRotation`)))
  ; IA_Movement
  (:`Triggered`
    (if (and (not (`self.IsHitting`)) (not (`self.IsDead`)))
      (`self.AddMovementInput` (`KismetMathLibrary.GetRightVector` (`KismetMathLibrary.MakeRotator` _returnvalue_roll 0.0 _returnvalue_yaw)) ActionValue_X)
      (`self.AddMovementInput` (`KismetMathLibrary.GetForwardVector` (`KismetMathLibrary.MakeRotator` 0.0 0.0 _returnvalue_yaw_2)) ActionValue_Y))))

(event `EnhancedInput|/Game/PathfinderContent/Player/Murdock/Input/IA_Sprint`
  (params (ActionValue :type Boolean) (ElapsedSeconds :type "Float (double-precision)") (TriggeredSeconds :type "Float (double-precision)") (InputAction :type "InputAction Object Reference" :default "/Game/PathfinderContent/Player/Murdock/Input/IA_Sprint.IA_Sprint"))
  (bind _charactermovement (`self.CharacterMovement`))
  ; IA_Sprint
  (:`Triggered`
    (set `CharacterMovementComponent.MaxWalkSpeed` 600.0 _charactermovement)
    (if (<= (`KismetMathLibrary.VSize` (`MovementComponent.Velocity` (`self.CharacterMovement`))) 0.0)
      (set `self.IsSprinting` false :!label _label)
      (else
        (set `self.IsSprinting` true))))
  (:`Completed`
    (set `CharacterMovementComponent.MaxWalkSpeed` 450.0 _charactermovement)
    (goto _label)))

(event `self.ReceiveAnyDamage`
  (params (Damage :type "Float (single-precision)") (DamageType :type "DamageType Object Reference") (InstigatedBy :type "Controller Object Reference") (DamageCauser :type "Actor Object Reference"))
  ; Event AnyDamage
  (set `self.IsHitting` true)
  (bind _output_get (`/Game/PathfinderContent/Component/BPC_StatSystem.DecreaseHealth` (`self.BPC_StatSystem`) Damage (`/Game/PathfinderContent/Player/Murdock/BP_MurdockController.PlayerHUD` (`self.PlayerController`))))
  (if _output_get
    (`GameplayStatics.PlaySoundAtLocation` "/Game/PathfinderContent/Player/Murdock/Sound/Murdock_Effort_Death.Murdock_Effort_Death" (0.0 0.0 0.0) (struct) 1.0 1.0 0.0 null null null null)
    (set `self.IsDead` true)
    (set `self.IsHitting` false)
    (`KismetSystemLibrary.Delay` 1.0)
    (`PrimitiveComponent.SetCollisionEnabled` (`self.CapsuleComponent`) "NoCollision")
    (`KismetSystemLibrary.Delay` 3.0)
    (`self.K2_DestroyActor`)
    (else
      (`GameplayStatics.PlaySoundAtLocation` "/Game/PathfinderContent/Player/Murdock/Sound/Murdock_Effort_Ability_Primary.Murdock_Effort_Ability_Primary" (0.0 0.0 0.0) (struct) 1.0 1.0 0.0 null null null null)
      (`|PlayMontage` (`self.Mesh`) "/Game/PathfinderContent/Player/Murdock/Animation/HitReact_A_Montage.HitReact_A_Montage"
        (:`then`
          (`KismetSystemLibrary.Delay` 1.0)
          (set `self.IsHitting` false))))))

(event `ZoomByAiming`
  ; IA_Zoom
  (set `self.IsSprinting` false)
  (bind (_direction _springarmlength _cameraylocation) (`Timeline|Timeline` :!label _label_2)
    (:`Update`
      (set `SpringArmComponent.TargetArmLength` _springarmlength (`self.SpringArm`))
      (`SceneComponent.K2_SetRelativeLocation` (`self.Camera`) (`KismetMathLibrary.MakeVector` 0.0 _cameraylocation) false false))))

(event `ZoomOutByAimingEnd`
  ; IA_Zoom
  (goto _label_2 :!via `Reverse`))

(event `EnhancedInput|/Game/PathfinderContent/Player/Murdock/Input/IA_Reload`
  (params (ActionValue :type Boolean) (ElapsedSeconds :type "Float (double-precision)") (TriggeredSeconds :type "Float (double-precision)") (InputAction :type "InputAction Object Reference" :default "/Game/PathfinderContent/Player/Murdock/Input/IA_Reload.IA_Reload"))
  ; IA_Reload
  (:`Triggered`
    (`/Game/PathfinderContent/Component/BPC_AttackSystem.Reload` (`self.BPC_AttackSystem`))))

(event `EnhancedInput|/Game/PathfinderContent/Player/Murdock/Input/IA_Dash`
  (params (ActionValue :type Boolean) (ElapsedSeconds :type "Float (double-precision)") (TriggeredSeconds :type "Float (double-precision)") (InputAction :type "InputAction Object Reference" :default "/Game/PathfinderContent/Player/Murdock/Input/IA_Dash.IA_Dash"))
  ; IA_Dash
  (:`Started`
    (if (<= (`self.DashCullDownTimer`) 0.0)
      (set `self.DashCullDownTimer` 0.0) ; 쿨타임을 0으로 바꿔주고
      (bind _returnvalue (`|GetDataTableRow` "/Game/PathfinderContent/Player/Murdock/DT_MurdockSkillInformation.DT_MurdockSkillInformation" "Dash")
        (:`then`
          (set `self.DashCullDownTimer` (`.SkillCullDown_9_8BBB0F224E16563199676A9B62794612` (break `/Game/PathfinderContent/Player/Murdock/S_SkillInformation` _returnvalue)))
          (`ActorComponent.SetActive` (`self.NS_Dash`) true false)
          (`GameplayStatics.PlaySoundAtLocation` "/Game/PathfinderContent/Player/Murdock/Sound/Murdock_Effort_Attack_01_Dialogue_Cue.Murdock_Effort_Attack_01_Dialogue_Cue" (0.0 0.0 0.0) (struct) 1.0 1.0 0.0 null null null null)
          (`GameplayStatics.PlaySoundAtLocation` "/Game/PathfinderContent/Player/Murdock/Sound/dash.dash" (0.0 0.0 0.0) (struct) 1.0 1.0 0.0 null null null null)
          (bind (_direction _dashtimeline) (`Timeline|DashTimeline` :!via `PlayFromStart`)
            (:`Update`
              (`self.K2_AddActorWorldOffset` (* _dashtimeline (`self.GetActorForwardVector`) 100.0) true))
            (:`Finished`
              (`KismetSystemLibrary.Delay` 0.3)
              (`ActorComponent.Deactivate` (`self.NS_Dash`)))))))))

(event `self.ReceiveTick`
  (params (DeltaSeconds :type "Float (single-precision)"))
  (if (> (`self.DashCullDownTimer`) 0.0)
    (bind _output_get (set `self.DashCullDownTimer` (- (`self.DashCullDownTimer`) DeltaSeconds)))
    (bind _returnvalue (`|GetDataTableRow` "/Game/PathfinderContent/Player/Murdock/DT_MurdockSkillInformation.DT_MurdockSkillInformation" "Dash")
      (:`then`
        (bind ((`SkillName_7_8BB134B04B42225489D751B312BCE64A` _skillname) (`SkillCullDown_9_8BBB0F224E16563199676A9B62794612` _skillculldown)) (break `/Game/PathfinderContent/Player/Murdock/S_SkillInformation` _returnvalue))
        (`/Game/PathfinderContent/UI/WB_HUD.SetCullDownPercent` (`/Game/PathfinderContent/Player/Murdock/BP_MurdockController.PlayerHUD` (`self.PlayerController`)) _output_get _skillculldown _skillname)))))

(fn `UserConstructionScript`)